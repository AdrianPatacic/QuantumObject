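; BP_QuantumObject is an actor that moves to another location when the player stops looking at it.
; QuantumShift uses the player character's IsInFrontOfPlayer check and a last-frame flag to detect the moment it leaves view, then calls ChangePos.
; ChangePos teleports it to a random TargetPoints entry outside the player's view, recursively rerolling with no retry limit, and prints the chosen index.
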(event Custom|ChangePos
  (Variables|Default|SetRandomNumber (Math|Random|RandomIntegerinRange 0 (- (Utilities|Array|Length (Variables|Default|GetTargetPoints)) 1)))
  (bind _isinfront (Default|IsinFrontOfPlayer (Variables|Default|GetPlayer) (Utilities|Array|Get(acopy) (Variables|Default|GetTargetPoints) (Variables|Default|GetRandomNumber))))
  (if (not _isinfront)
    (Transformation|SetActorLocation (Transformation|GetActorLocation (Utilities|Array|Get(acopy) (Variables|Default|GetTargetPoints) (Variables|Default|GetRandomNumber))) false false)
    (Development|PrintString (Utilities|String|ToString(Integer) (Variables|Default|GetRandomNumber)))
    (else
      (CallFunction|ChangePos))))

(event EventBeginPlay
  (bind _asbp_first_person_character (Utilities|Casting|CastToBP_FirstPersonCharacter (Game|Player|GetPlayerPawn 0)))
  (Variables|Default|SetPlayer _asbp_first_person_character))

(fn ConstructionScript)

(fn QuantumShift
  (bind _isinfront (Default|IsinFrontOfPlayer (Variables|Default|GetPlayer) self))
  (if (and (not _isinfront) (Variables|Default|GetWasSeenLastFrame))
    (CallFunction|ChangePos)
    (Variables|Default|SetWasSeenLastFrame _isinfront)
    (else
      (Variables|Default|SetWasSeenLastFrame _isinfront))))